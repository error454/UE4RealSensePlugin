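; Player controller that drives the player pawn from camera head and face tracking through an Expression object, started on BeginPlay.
; Each tick, per-frame head deltas, filtered for jitter and outliers, accumulate into targets that interpolated pawn location and control rotation follow.
; The first detected head sets the baseline.
; Eye direction, mouth values and eyebrow values move or scale the matching HeadTrackingPawn face parts.
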(event EventTick
  (params (DeltaSeconds :type Float%20%28single-precision%29))
  (if (> (Variables|/Script/RealSensePlugin.ExpressionComponent|GetHeadCount (Variables|Default|GetExpression)) 0)
    (if (Variables|Default|GetHeadControl)
      (CallFunction|CalcPositionDifferential)
      (CallFunction|CalcRotationDifferential)
      (CallFunction|CalcEyesDirection)
      (CallFunction|CalcMouthScale)
      (CallFunction|CalcBrows)
      (Variables|Default|SetTargetPosition (+ (Variables|Default|GetTargetPosition) (Variables|Default|GetPositionDifferential)))
      (bind _output_get (Variables|Default|SetCurrentPosition (Math|Interpolation|VInterpTo (Variables|Default|GetCurrentPosition) (Variables|Default|GetTargetPosition) (Utilities|Time|GetWorldDeltaSeconds) (Variables|Default|GetInterpolationSpeed))))
      (Transformation|SetActorLocation (Game|Player|GetPlayerPawn 0) _output_get false false)
      (Variables|Default|SetBaseHeadPosition (Variables|/Script/RealSensePlugin.ExpressionComponent|GetHeadPosition (Variables|Default|GetExpression)))
      (Variables|Default|SetTargetRotation (Math|Rotator|CombineRotators (Variables|Default|GetTargetRotation) (Variables|Default|GetRotationDifferential)))
      (bind _output_get_2 (Variables|Default|SetCurrentRotation (Math|Interpolation|RInterpTo (Variables|Default|GetCurrentRotation) (Variables|Default|GetTargetRotation) (Utilities|Time|GetWorldDeltaSeconds) (Variables|Default|GetInterpolationSpeed))))
      (Pawn|SetControlRotation _output_get_2)
      (Variables|Default|SetBaseHeadRotation (Variables|/Script/RealSensePlugin.ExpressionComponent|GetHeadRotation (Variables|Default|GetExpression)))
      (else
        (CallFunction|SetupHeadControl)))))

(event EventEndPlay
  (params (EndPlayReason :type EEndPlayReason%20Enum :default "Destroyed"))
  (Class|RealSenseComponent|StopCamera (Variables|Default|GetExpression)))

(event EventBeginPlay
  (Class|RealSenseComponent|StartCamera (Variables|Default|GetExpression)))

(fn ConstructionScript)

(fn SetupHeadControl
  (Variables|Default|SetBaseHeadPosition (Variables|/Script/RealSensePlugin.ExpressionComponent|GetHeadPosition (Variables|Default|GetExpression)))
  (bind _output_get (Variables|Default|SetCurrentPosition (Transformation|GetActorLocation (Game|Player|GetPlayerPawn 0))))
  (Variables|Default|SetTargetPosition _output_get)
  (Variables|Default|SetBaseHeadRotation (Variables|/Script/RealSensePlugin.ExpressionComponent|GetHeadRotation (Variables|Default|GetExpression)))
  (bind _output_get_2 (Variables|Default|SetCurrentRotation (Pawn|GetControlRotation :!class /Script/Engine.Controller)))
  (Variables|Default|SetTargetRotation _output_get_2)
  (Variables|Default|SetEyeDirection (* (Variables|/Script/RealSensePlugin.ExpressionComponent|GetEyesDirection (Variables|Default|GetExpression)) 2e+02))
  (Variables|Default|SetHeadControl true)
  (return))

(fn CalcPositionDifferential
  (bind _expression (Variables|Default|GetExpression))
  (bind _baseheadposition (Variables|Default|GetBaseHeadPosition))
  (bind _headposition (Variables|/Script/RealSensePlugin.ExpressionComponent|GetHeadPosition _expression))
  (bind _returnvalue (- _headposition _baseheadposition))
  (LocalVariables|SetX (* (.z _returnvalue) -1.0))
  (LocalVariables|SetY (* (.x _returnvalue) -1.0))
  (LocalVariables|SetZ (.y _returnvalue))
  (if (or (< (Math|Float|Absolute(Float) (LocalVariables|GetX)) 5.0) (> (Math|Float|Absolute(Float) (LocalVariables|GetX)) 1e+02))
    (LocalVariables|SetX 0.0))
  (if (or (< (Math|Float|Absolute(Float) (LocalVariables|GetY)) 5.0) (> (Math|Float|Absolute(Float) (LocalVariables|GetY)) 1e+02))
    (LocalVariables|SetY 0.0))
  (if (or (< (Math|Float|Absolute(Float) (LocalVariables|GetZ)) 5.0) (> (Math|Float|Absolute(Float) (LocalVariables|GetZ)) 1e+02))
    (LocalVariables|SetZ 0.0))
  (Variables|Default|SetPositionDifferential (* (Math|Vector|MakeVector (LocalVariables|GetX) (LocalVariables|GetY) (LocalVariables|GetZ)) 2.0))
  (return))

(fn CalcRotationDifferential
  (bind _expression (Variables|Default|GetExpression))
  (bind _baseheadrotation (Variables|Default|GetBaseHeadRotation))
  (bind _headrotation (Variables|/Script/RealSensePlugin.ExpressionComponent|GetHeadRotation _expression))
  (bind _returnvalue (Math|Rotator|Delta(Rotator) _headrotation _baseheadrotation))
  (LocalVariables|SetRoll (.roll _returnvalue))
  (LocalVariables|SetPitch (.pitch _returnvalue))
  (LocalVariables|SetYaw (.yaw _returnvalue))
  (if (or (< (Math|Float|Absolute(Float) (LocalVariables|GetRoll)) 1.0) (> (Math|Float|Absolute(Float) (LocalVariables|GetRoll)) 1e+02))
    (LocalVariables|SetRoll 0.0))
  (if (or (< (Math|Float|Absolute(Float) (LocalVariables|GetPitch)) 1.0) (> (Math|Float|Absolute(Float) (LocalVariables|GetPitch)) 1e+02))
    (LocalVariables|SetPitch 0.0))
  (if (or (< (Math|Float|Absolute(Float) (LocalVariables|GetYaw)) 1.0) (> (Math|Float|Absolute(Float) (LocalVariables|GetYaw)) 1e+02))
    (LocalVariables|SetYaw 0.0))
  (Variables|Default|SetRotationDifferential (Math|Rotator|MakeRotator (LocalVariables|GetRoll) (LocalVariables|GetPitch) (LocalVariables|GetYaw)))
  (return))

(fn CalcEyesDirection
  (bind _output_get (Variables|Default|SetEyeDirection (* (Variables|/Script/RealSensePlugin.ExpressionComponent|GetEyesDirection (Variables|Default|GetExpression)) 3e+01)))
  (bind _ashead_tracking_pawn (Utilities|Casting|CastToHeadTrackingPawn (Game|Player|GetPlayerPawn 0)))
  (bind _eyebox (Default|GetEyeBoxL _ashead_tracking_pawn))
  (Transformation|SetRelativeLocation _eyebox (Math|Vector|MakeVector (.z _output_get) (.x _output_get) (.y _output_get)) false false)
  (bind _eyebox_2 (Default|GetEyeBoxR _ashead_tracking_pawn))
  (Transformation|SetRelativeLocation _eyebox_2 (Math|Vector|MakeVector (.z _output_get) (.x _output_get) (.y _output_get)) false false))

(fn CalcMouthScale
  (bind _ashead_tracking_pawn (Utilities|Casting|CastToHeadTrackingPawn (Game|Player|GetPlayerPawn 0)))
  (bind _mouth (Default|GetMouthRoot _ashead_tracking_pawn))
  (Transformation|SetRelativeScale3D _mouth (Math|Vector|MakeVector (/ (Math|Float|Clamp(Float) (Variables|/Script/RealSensePlugin.ExpressionComponent|GetMouthOpen (Variables|Default|GetExpression)) 1e+01 1e+02) 1e+02) (/ (Math|Float|Clamp(Float) (Variables|/Script/RealSensePlugin.ExpressionComponent|GetMouthSmile (Variables|Default|GetExpression)) 1e+01 1e+02) 1e+02) (/ (Math|Float|Clamp(Float) (Variables|/Script/RealSensePlugin.ExpressionComponent|GetMouthKiss (Variables|Default|GetExpression)) 1e+01 1e+02) 1e+02))))

(fn CalcBrows
  (bind _expression (Variables|Default|GetExpression))
  (bind _ashead_tracking_pawn (Utilities|Casting|CastToHeadTrackingPawn (Game|Player|GetPlayerPawn 0)))
  (bind _browleft (Default|GetBrowLeft _ashead_tracking_pawn))
  (Transformation|SetRelativeLocation _browleft (Math|Vector|MakeVector 0.0 0.0 (* (Variables|/Script/RealSensePlugin.ExpressionComponent|GetEyebrowLeft _expression) -1.0)) false false)
  (bind _browright (Default|GetBrowRight _ashead_tracking_pawn))
  (Transformation|SetRelativeLocation _browright (Math|Vector|MakeVector 0.0 0.0 (* (Variables|/Script/RealSensePlugin.ExpressionComponent|GetEyebrowRight _expression) -1.0)) false false))