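; HeadTrackingPawn is a RealSense head-tracking pawn Blueprint that exposes the parts of a face.
; Five getter functions return the left and right eye boxes, the mouth root and the left and right brows.
; The event graph and construction script are empty, so the Blueprint itself contains no tracking or animation logic.
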(event EventBeginPlay)

(event EventActorBeginOverlap
  (params (OtherActor :type Actor%20Object%20Reference)))

(event EventTick
  (params (DeltaSeconds :type Float%20%28single-precision%29)))

(fn ConstructionScript)

(fn GetEyeBoxL
  (return (Variables|Default|GetEyeBoxL)))

(fn GetEyeBoxR
  (return (Variables|Default|GetEyeBoxR)))

(fn GetMouthRoot
  (return (Variables|Default|GetMouth)))

(fn GetBrowLeft
  (return (Variables|Default|GetbrowL)))

(fn GetBrowRight
  (return (Variables|Default|GetbrowR)))