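; Player controller that drives the player pawn's location and control rotation from RealSense head tracking, running the camera from BeginPlay to EndPlay.
; The first tick with a detected head captures baselines from the head, pawn and control rotation.
; Later tracked ticks add frame-to-frame head deltas to targets, zeroing jitter and outliers per axis and remapping and scaling position.
; Pawn location and control rotation interpolate toward those targets.
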(event EventTick
  (params (DeltaSeconds :type Float%20%28single-precision%29))
  (if (> (Variables|/Script/RealSensePlugin.HeadTrackingComponent|GetHeadCount (Variables|Default|GetHeadTracking)) 0)
    (if (Variables|Default|GetHeadControl)
      (CallFunction|CalcPositionDifferential)
      (CallFunction|CalcRotationDifferential)
      (Variables|Default|SetTargetPosition (+ (Variables|Default|GetTargetPosition) (Variables|Default|GetPositionDifferential)))
      (bind _output_get (Variables|Default|SetCurrentPosition (Math|Interpolation|VInterpTo (Variables|Default|GetCurrentPosition) (Variables|Default|GetTargetPosition) (Utilities|Time|GetWorldDeltaSeconds) (Variables|Default|GetInterpolationSpeed))))
      (Transformation|SetActorLocation (Game|Player|GetPlayerPawn 0) _output_get false false)
      (Variables|Default|SetBaseHeadPosition (Variables|/Script/RealSensePlugin.HeadTrackingComponent|GetHeadPosition (Variables|Default|GetHeadTracking)))
      (Variables|Default|SetTargetRotation (Math|Rotator|CombineRotators (Variables|Default|GetTargetRotation) (Variables|Default|GetRotationDifferential)))
      (bind _output_get_2 (Variables|Default|SetCurrentRotation (Math|Interpolation|RInterpTo (Variables|Default|GetCurrentRotation) (Variables|Default|GetTargetRotation) (Utilities|Time|GetWorldDeltaSeconds) (Variables|Default|GetInterpolationSpeed))))
      (Pawn|SetControlRotation _output_get_2)
      (Variables|Default|SetBaseHeadRotation (Variables|/Script/RealSensePlugin.HeadTrackingComponent|GetHeadRotation (Variables|Default|GetHeadTracking)))
      (else
        (CallFunction|SetupHeadControl)))))

(event EventEndPlay
  (params (EndPlayReason :type EEndPlayReason%20Enum :default "Destroyed"))
  (Class|RealSenseComponent|StopCamera (Variables|Default|GetHeadTracking)))

(event EventBeginPlay
  (Class|RealSenseComponent|StartCamera (Variables|Default|GetHeadTracking)))

(fn ConstructionScript)

(fn SetupHeadControl
  (Variables|Default|SetBaseHeadPosition (Variables|/Script/RealSensePlugin.HeadTrackingComponent|GetHeadPosition (Variables|Default|GetHeadTracking)))
  (bind _output_get (Variables|Default|SetCurrentPosition (Transformation|GetActorLocation (Game|Player|GetPlayerPawn 0))))
  (Variables|Default|SetTargetPosition _output_get)
  (Variables|Default|SetBaseHeadRotation (Variables|/Script/RealSensePlugin.HeadTrackingComponent|GetHeadRotation (Variables|Default|GetHeadTracking)))
  (bind _output_get_2 (Variables|Default|SetCurrentRotation (Pawn|GetControlRotation :!class /Script/Engine.Controller)))
  (Variables|Default|SetTargetRotation _output_get_2)
  (Variables|Default|SetHeadControl true)
  (return))

(fn CalcPositionDifferential
  (bind _headtracking (Variables|Default|GetHeadTracking))
  (bind _baseheadposition (Variables|Default|GetBaseHeadPosition))
  (bind _headposition (Variables|/Script/RealSensePlugin.HeadTrackingComponent|GetHeadPosition _headtracking))
  (bind _returnvalue (- _headposition _baseheadposition))
  (LocalVariables|SetX (* (.z _returnvalue) -1.0))
  (LocalVariables|SetY (* (.x _returnvalue) -1.0))
  (LocalVariables|SetZ (.y _returnvalue))
  (if (or (< (Math|Float|Absolute(Float) (LocalVariables|GetX)) 5.0) (> (Math|Float|Absolute(Float) (LocalVariables|GetX)) 1e+02))
    (LocalVariables|SetX 0.0))
  (if (or (< (Math|Float|Absolute(Float) (LocalVariables|GetY)) 5.0) (> (Math|Float|Absolute(Float) (LocalVariables|GetY)) 1e+02))
    (LocalVariables|SetY 0.0))
  (if (or (< (Math|Float|Absolute(Float) (LocalVariables|GetZ)) 5.0) (> (Math|Float|Absolute(Float) (LocalVariables|GetZ)) 1e+02))
    (LocalVariables|SetZ 0.0))
  (Variables|Default|SetPositionDifferential (* (Math|Vector|MakeVector (LocalVariables|GetX) (LocalVariables|GetY) (LocalVariables|GetZ)) 2.0))
  (return))

(fn CalcRotationDifferential
  (bind _headtracking (Variables|Default|GetHeadTracking))
  (bind _baseheadrotation (Variables|Default|GetBaseHeadRotation))
  (bind _headrotation (Variables|/Script/RealSensePlugin.HeadTrackingComponent|GetHeadRotation _headtracking))
  (bind _returnvalue (Math|Rotator|Delta(Rotator) _headrotation _baseheadrotation))
  (LocalVariables|SetRoll (.roll _returnvalue))
  (LocalVariables|SetPitch (.pitch _returnvalue))
  (LocalVariables|SetYaw (.yaw _returnvalue))
  (if (or (< (Math|Float|Absolute(Float) (LocalVariables|GetRoll)) 1.0) (> (Math|Float|Absolute(Float) (LocalVariables|GetRoll)) 1e+02))
    (LocalVariables|SetRoll 0.0))
  (if (or (< (Math|Float|Absolute(Float) (LocalVariables|GetPitch)) 1.0) (> (Math|Float|Absolute(Float) (LocalVariables|GetPitch)) 1e+02))
    (LocalVariables|SetPitch 0.0))
  (if (or (< (Math|Float|Absolute(Float) (LocalVariables|GetYaw)) 1.0) (> (Math|Float|Absolute(Float) (LocalVariables|GetYaw)) 1e+02))
    (LocalVariables|SetYaw 0.0))
  (Variables|Default|SetRotationDifferential (Math|Rotator|MakeRotator (LocalVariables|GetRoll) (LocalVariables|GetPitch) (LocalVariables|GetYaw)))
  (return))